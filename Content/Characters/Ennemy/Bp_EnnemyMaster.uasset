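; Master enemy character Blueprint that handles health, damage feedback and death.
; Each hit spawns a UI_Hit_Feedback actor above the enemy showing the damage, then subtracts it from Health.
; At zero health it stops movement, ragdolls the mesh, decrements EnemyAlive on GameMode_Gruttin and calls MobCheck, then destroys itself after a short delay.
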(event `self.ReceiveBeginPlay`
  (set `self.Health` (`self.MaxHealth`))
  (bind _asgame_mode_gruttin (cast `/Game/GameMode_Gruttin` (`GameplayStatics.GetGameMode`)))
  (set `self.As Game Mode Gruttin` _asgame_mode_gruttin))

(event `/Game/Characters/IBP_Damage.Damage`
  (params (Target :type "Object Object Reference") (Damage :type "Float (double-precision)"))
  (bind _returnvalue_location (`KismetMathLibrary.BreakTransform` (`self.GetTransform`)))
  (if (not (`self.Death?`))
    (bind _returnvalue (`|SpawnActorFromClass` "/Game/UI/UI_Hit_Feedback.UI_Hit_Feedback_C" (`KismetMathLibrary.MakeTransform` (`KismetMathLibrary.MakeVector` (.x _returnvalue_location) (.y _returnvalue_location) (+ (.z _returnvalue_location) 50.0))) "Undefined" "MultiplyWithRoot" null null))
    (`/Game/UI/UI_Hit_Feedback.HItP` _returnvalue Damage)
    (bind _output_get (set `self.Health` (- (`self.Health`) Damage)))
    (if (<= _output_get 0.0)
      (`self.Death`))))

(event `Death`
  (bind _as_game_mode_gruttin (`self.As Game Mode Gruttin`))
  (bind _mesh (`self.Mesh`))
  (if (not (`self.Death?`))
    (set `self.Death?` true)
    (`MovementComponent.StopMovementImmediately` (`self.CharacterMovement`))
    (`PrimitiveComponent.SetSimulatePhysics` _mesh true)
    (`PrimitiveComponent.SetCollisionObjectType` _mesh "ECC_WorldDynamic")
    (`PrimitiveComponent.SetCollisionEnabled` _mesh "QueryAndPhysics")
    (`/Engine/EditorBlueprintResources/StandardMacros.DecrementInt` (`/Game/GameMode_Gruttin.Enemy_Alive` _as_game_mode_gruttin)
      (:`  `
        (`/Game/GameMode_Gruttin.Mob_Check` _as_game_mode_gruttin)
        (`KismetSystemLibrary.Delay` 3.0)
        (`self.K2_DestroyActor`)))))

(fn `UserConstructionScript`)