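; BP_Goal is the goal actor that loses health when enemies reach it.
; When a Bp_EnnemyMaster overlaps its Cube, it calls that enemy's Death and subtracts a fixed amount from HealthGoal on GameMode_Gruttin, cached at BeginPlay.
; When health exactly equals zero, it shows UI_GameOver, pauses the game and switches to UI-only input with a visible cursor.
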(event `self.ReceiveBeginPlay`
  (bind _asgame_mode_gruttin (cast `/Game/GameMode_Gruttin` (`GameplayStatics.GetGameMode`)))
  (set `self.As Game Mode Gruttin` _asgame_mode_gruttin))

(event `self.Cube.OnComponentBeginOverlap`
  (params (OverlappedComponent :type "PrimitiveComponent Object Reference") (OtherActor :type "Actor Object Reference") (OtherComp :type "PrimitiveComponent Object Reference") (OtherBodyIndex :type Integer) (bFromSweep :type Boolean) (SweepResult :type "HitResult Structure (by ref)"))
  (bind _returnvalue (`GameplayStatics.GetPlayerController` 0))
  (bind _as_game_mode_gruttin (`self.As Game Mode Gruttin`))
  (bind _health_goal (`/Game/GameMode_Gruttin.Health_Goal` _as_game_mode_gruttin))
  (bind _asbp_ennemy_master (cast `/Game/Characters/Ennemy/Bp_EnnemyMaster` OtherActor))
  (`/Game/Characters/Ennemy/Bp_EnnemyMaster.Death` _asbp_ennemy_master)
  (set `/Game/GameMode_Gruttin.Health_Goal` (- _health_goal 10.0) _as_game_mode_gruttin)
  (if (== _health_goal 0.0)
    (bind _returnvalue_2 (`|CreateWidget` "/Game/UI/UI_GameOver.UI_GameOver_C"))
    (`UserWidget.AddToViewport` _returnvalue_2 0)
    (`GameplayStatics.SetGamePaused` true)
    (set `PlayerController.bShowMouseCursor` true _returnvalue)
    (`WidgetBlueprintLibrary.SetInputMode_UIOnlyEx` _returnvalue null)))

(fn `UserConstructionScript`)