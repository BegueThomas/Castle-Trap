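; Trap build system for the player's BP_Gruttin pawn, with a toggled build mode and mouse-wheel selection from DT_BuildParts.
; A ghost mesh follows the pawn's trace, colored green or red by resource cost and placement validity, including multi-trace ground checks for floor-only parts.
; Placing spawns the part's Blueprint and passes its price to BP_BuildMaster.
; Holding destroy starts the pawn's repair progress; the Repair event refunds and destroys the targeted part.
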(event `ResetBuildMode`
  ; Preview du trap en jeu
  (goto _label :!via `Reset`))

(event `Preview_loop`
  (params (HitResult :type "HitResult Structure") (ReturnValue :type Boolean))
  (bind (_bblockinghit _binitialoverlap _time _distance _location _impactpoint _normal _impactnormal _physmat _hitactor _hitcomponent _hitbonename _bonename _hititem _elementindex _faceindex _tracestart _traceend) (`GameplayStatics.BreakHitResult` HitResult))
  (bind _preview_mesh (`self.Preview_Mesh`))
  (bind (_returnvalue_roll _returnvalue_pitch _returnvalue_yaw) (`KismetMathLibrary.BreakRotator` (`Actor.K2_GetActorRotation` _hitactor)))
  (bind (_name _mesh _blueprint _layer_trace_channel _price) (break `/Game/Enviro/Trap/S_BuildParts` (`|GetArrayItem` (`self.DT_BuildParts`) (`self.Build_Index`))))
  ; Preview du trap en jeu
  (if ReturnValue
    (`|ExecutionSequence`
      (:`then_0`
        (`/Engine/EditorBlueprintResources/StandardMacros.DoOnce` false :!label _label
          (:`Completed`
            (bind _returnvalue (`|AddComponentByClass` (`self.As BP Gruttin`) "/Script/Engine.StaticMeshComponent" false (`self.BuildPreviewTransform`)))
            (bind _output_get (set `self.Preview_Mesh` _returnvalue))
            (`StaticMeshComponent.SetStaticMesh` _output_get _mesh))))
      (:`then_1`
        (bind _output_get_2 (set `self.BuildPreviewTransform` (`KismetMathLibrary.MakeTransform` _location (`KismetMathLibrary.MakeRotator` _returnvalue_roll _returnvalue_pitch _returnvalue_yaw))))
        (`SceneComponent.K2_SetWorldTransform` (`self.Preview_Mesh`) _output_get_2 false false))
      (:`then_2`
        (if (>= (`/Game/Characters/Gruttin/BP_Gruttin.HeldRessource` (`self.As BP Gruttin`)) _price) :!label _label_2
          (if (`self.CanBuild?`)
            (`PrimitiveComponent.SetMaterial` _preview_mesh 0 "/Game/Enviro/Trap/Visual/mat_ghost_green.mat_ghost_green")
            (else
              (`PrimitiveComponent.SetMaterial` _preview_mesh 0 "/Game/Enviro/Trap/Visual/mat_ghost_red.mat_ghost_red" :!label _label_3)))
          (else
            (goto _label_3)))
        (`PrimitiveComponent.SetCollisionEnabled` _preview_mesh "NoCollision")))
    (else
      (`|ExecutionSequence`
        (:`then_0`
          (goto _label))
        (:`then_1`
          (goto _label_2))
        (:`then_2`
          (bind (_outhit _returnvalue_2) (`KismetSystemLibrary.LineTraceSingle` _traceend (`KismetMathLibrary.MakeVector` (.x _traceend) (.y _traceend) (- (.z _traceend) 200.0)) "TraceTypeQuery1"))
          (bind (_bblockinghit_2 _binitialoverlap_2 _time_2 _distance_2 _location_2 _impactpoint_2 _normal_2 _impactnormal_2 _physmat_2 _hitactor_2) (`GameplayStatics.BreakHitResult` _outhit))
          (`/Engine/EditorBlueprintResources/StandardMacros.IsValid` _hitactor_2
            (:`Is Valid`
              (bind _output_get_3 (set `self.BuildPreviewTransform` (`KismetMathLibrary.MakeTransform` _location_2 (`Actor.K2_GetActorRotation` _hitactor_2))))
              (`SceneComponent.K2_SetWorldTransform` (`self.Preview_Mesh`) _output_get_3 false false))))))))

(event `self.ReceiveBeginPlay`
  (bind _asbp_gruttin (cast `/Game/Characters/Gruttin/BP_Gruttin` (`GameplayStatics.GetPlayerPawn` 0)))
  (bind _output_get (set `self.As BP Gruttin` _asbp_gruttin))
  (set `self.Camera` (`/Game/Characters/Gruttin/BP_Gruttin.Camera` _output_get))
  (bind _outrownames (`DataTableFunctionLibrary.GetDataTableRowNames` "/Game/Enviro/Trap/DT_BuildParts.DT_BuildParts"))
  (for _array_element _outrownames
    (bind _returnvalue (`|GetDataTableRow` "/Game/Enviro/Trap/DT_BuildParts.DT_BuildParts" _array_element)
      (:`then`
        (`KismetArrayLibrary.Array_Add` (`self.DT_BuildParts`) _returnvalue)
        (`SceneComponent.SetVisibility` (`/Game/Characters/Gruttin/BP_Gruttin.book` (`self.As BP Gruttin`)) false true)))))

(event `self.ReceiveTick`
  (params (DeltaSeconds :type "Float (single-precision)"))
  (bind _buildpreviewtransform_location (`KismetMathLibrary.BreakTransform` (`self.BuildPreviewTransform`)))
  (bind _as_bp_gruttin (`self.As BP Gruttin`))
  (bind _out_hit (`/Game/Characters/Gruttin/BP_Gruttin.Out Hit` _as_bp_gruttin))
  (bind (_bblockinghit _binitialoverlap _time _distance _location _impactpoint _normal _impactnormal _physmat _hitactor) (`GameplayStatics.BreakHitResult` _out_hit))
  ; Comment
  (if (`self.InBuildMode?`)
    (`self.Preview_loop` _out_hit (`/Game/Characters/Gruttin/BP_Gruttin.Value` _as_bp_gruttin)))
  (switch `/Game/Enviro/Trap/E_TrapType` (`.Position_22_D07D5B6E4B583807788A4EA0832D451B` (break `/Game/Enviro/Trap/S_BuildParts` (`|GetArrayItem` (`self.DT_BuildParts`) (`self.Build_Index`))))
    (:`NewEnumerator0`
      (if (`KismetSystemLibrary.DoesImplementInterface` _hitactor "/Game/Enviro/Trap/Blueprints/IBP_SeeStat.IBP_SeeStat_C") :!label _label_4
        (bind _last_seen (`self.last_seen` :!label _label_5)
          (:`then`
            (message `/Game/Enviro/Trap/Blueprints/IBP_SeeStat.OnObjectUntargeted` _last_seen))
          (:`else`
            _))
        (bind _asbp_build_master (cast `/Game/Enviro/Trap/Blueprints/BP_BuildMaster` _hitactor)
          (:`then`
            (set `self.last_seen` _asbp_build_master)
            (`/Game/Enviro/Trap/Blueprints/BP_BuildMaster.OnObjectTargeted` _asbp_build_master))
          (:`CastFailed`
            _))
        (set `self.CanBuild?` false)
        (elif (`KismetSystemLibrary.DoesImplementInterface` _hitactor "/Game/Characters/Gruttin/IBP_Interact.IBP_Interact_C")
          (goto _label_5)
          (else
            (bind _last_seen_2 (`self.last_seen`)
              (:`then`
                (message `/Game/Enviro/Trap/Blueprints/IBP_SeeStat.OnObjectUntargeted` _last_seen_2))
              (:`else`
                _))
            (set `self.CanBuild?` true)))))
    (:`NewEnumerator1`
      (for _array_element (`self.Verify_Floor`)
        (bind _returnvalue (+ _array_element _buildpreviewtransform_location))
        (bind (_outhit _returnvalue_2) (`KismetSystemLibrary.LineTraceSingle` :`Start` _returnvalue :`End` (`KismetMathLibrary.MakeVector` (.x _returnvalue) (.y _returnvalue) (+ (.z _returnvalue) -5.0)) :`TraceChannel` "TraceTypeQuery1" :`DrawDebugType` "ForOneFrame"))
        (if _returnvalue_2
          (set `self.Verify_index` (+ (`self.Verify_index`) 1))
          (else
            (set `self.Verify_index` (- (`self.Verify_index`) 1)))))
      (if (== (`self.Verify_index`) (`KismetArrayLibrary.Array_Length` (`self.Verify_Floor`)))
        (set `self.Verify_index` 0)
        (goto _label_4)
        (else
          (set `self.Verify_index` 0)
          (goto _label_5))))))

(event `EnhancedInput|/Game/Characters/Gruttin/Action/IA_Build`
  (params (ActionValue :type Boolean) (ElapsedSeconds :type "Float (double-precision)") (TriggeredSeconds :type "Float (double-precision)") (InputAction :type "InputAction Object Reference" :default "/Game/Characters/Gruttin/Action/IA_Build.IA_Build"))
  (bind _as_bp_gruttin (`self.As BP Gruttin`))
  (bind _book (`/Game/Characters/Gruttin/BP_Gruttin.book` _as_bp_gruttin))
  (bind _set_text (`/Game/UI/UI_Gruttin.Set_Text` (`/Game/Characters/Gruttin/BP_Gruttin.Ui_Gruttin` _as_bp_gruttin)))
  ; Activation / désactivation du mode hack
  (:`Started`
    (if (not (`self.InBuildMode?`))
      (set `self.InBuildMode?` true)
      (set `Widget.Visibility` "Visible" _set_text)
      (`SceneComponent.SetVisibility` _book true true)
      (else
        (set `self.InBuildMode?` false :!label _label_6)
        (bind _preview_mesh (`self.Preview_Mesh`)
          (:`then`
            _)
          (:`else`
            _))
        (`StaticMeshComponent.SetStaticMesh` _preview_mesh null)
        (set `self.Preview_Mesh` null)
        (`self.ResetBuildMode`)
        (`SceneComponent.SetVisibility` _book false true)
        (set `Widget.Visibility` "Hidden" _set_text)))))

(event `StopBuildMode`
  ; Activation / désactivation du mode hack
  (goto _label_6))

(event `EnhancedInput|/Game/Characters/Gruttin/Action/IA_PlaceBuild`
  (params (ActionValue :type Boolean) (ElapsedSeconds :type "Float (double-precision)") (TriggeredSeconds :type "Float (double-precision)") (InputAction :type "InputAction Object Reference" :default "/Game/Characters/Gruttin/Action/IA_PlaceBuild.IA_PlaceBuild"))
  (bind (_name _mesh _blueprint _layer_trace_channel _price) (break `/Game/Enviro/Trap/S_BuildParts` (`|GetArrayItem` (`self.DT_BuildParts`) (`self.Build_Index`))))
  (:`Started`
    (if (`self.InBuildMode?`)
      (if (`self.CanBuild?`)
        (if (>= (`/Game/Characters/Gruttin/BP_Gruttin.HeldRessource` (`self.As BP Gruttin`)) _price)
          (bind _returnvalue (`|SpawnActorFromClass` _blueprint (`self.BuildPreviewTransform`) "DontSpawnIfColliding" "MultiplyWithRoot" null null))
          (bind _asbp_build_master (cast `/Game/Enviro/Trap/Blueprints/BP_BuildMaster` _returnvalue))
          (`/Game/Enviro/Trap/Blueprints/BP_BuildMaster.Spawn` _asbp_build_master _price))))))

(event `EnhancedInput|/Game/Characters/Gruttin/Action/IA_Destroy`
  (params (ActionValue :type Boolean) (ElapsedSeconds :type "Float (double-precision)") (TriggeredSeconds :type "Float (double-precision)") (InputAction :type "InputAction Object Reference" :default "/Game/Characters/Gruttin/Action/IA_Destroy.IA_Destroy"))
  (bind _as_bp_gruttin (`self.As BP Gruttin`))
  (bind _as_bp_gruttin_2 (`self.As BP Gruttin`))
  (bind _progress_repair (`/Game/Characters/Gruttin/BP_Gruttin.Progress_repair` _as_bp_gruttin))
  (bind _progressbar_0 (`/Game/UI/UI_Gruttin.ProgressBar_0` (`/Game/Characters/Gruttin/BP_Gruttin.Ui_Gruttin` _as_bp_gruttin)))
  (:`Started`
    (if (`/Game/Characters/Gruttin/BP_Gruttin.Value` _as_bp_gruttin_2)
      (if (`Actor.ActorHasTag` (`.HitActor` (`GameplayStatics.BreakHitResult` (`/Game/Characters/Gruttin/BP_Gruttin.Out Hit` _as_bp_gruttin_2))) "Build")
        (`TimelineComponent.SetPlayRate` _progress_repair 1.0)
        (set `Widget.Visibility` "Visible" _progressbar_0)
        (`/Game/Characters/Gruttin/BP_Gruttin.Start_Repair` _as_bp_gruttin))))
  (:`Canceled`
    (`TimelineComponent.SetPlayRate` _progress_repair 10.0 :!label _label_7)
    (set `Widget.Visibility` "Hidden" _progressbar_0)
    (`/Game/Characters/Gruttin/BP_Gruttin.Cancel_Repair` _as_bp_gruttin))
  (:`Completed`
    (goto _label_7)))

(event `EnhancedInput|/Game/Characters/Gruttin/Action/IA_RotateBuild`
  (params (ActionValue :type Boolean) (ElapsedSeconds :type "Float (double-precision)") (TriggeredSeconds :type "Float (double-precision)") (InputAction :type "InputAction Object Reference" :default "/Game/Characters/Gruttin/Action/IA_RotateBuild.IA_RotateBuild"))
  (:`Started`
    (bind _returnvalue (`KismetSystemLibrary.K2_SetTimerDelegate` (delegate `RotatePreview`) 0.05 true))
    (set `self.RotateBuildPreview` _returnvalue))
  (:`Canceled`
    (`KismetSystemLibrary.K2_ClearAndInvalidateTimerHandle` (`self.RotateBuildPreview`) :!label _label_8)
    (set `self.RotateBuildPreview` (struct)))
  (:`Completed`
    (goto _label_8)))

(event `RotatePreview`
  (bind (_buildpreviewtransform_location _buildpreviewtransform_rotation) (`KismetMathLibrary.BreakTransform` (`self.BuildPreviewTransform`)))
  (set `self.BuildPreviewRotation` (`KismetMathLibrary.ComposeRotators` _buildpreviewtransform_rotation (struct :`Pitch` 0.05 :`Yaw` 0.05 :`Roll` 0.05)))
  (`KismetSystemLibrary.PrintString` "Hello"))

(event `Repair`
  (bind (_bblockinghit _binitialoverlap _time _distance _location _impactpoint _normal _impactnormal _physmat _hitactor) (`GameplayStatics.BreakHitResult` (`/Game/Characters/Gruttin/BP_Gruttin.Out Hit` (`self.As BP Gruttin`))))
  (for _array_element (`self.DT_BuildParts`)
    (bind (_name _mesh _blueprint _layer_trace_channel _price) (break `/Game/Enviro/Trap/S_BuildParts` _array_element))
    (if (== (`GameplayStatics.GetObjectClass` _hitactor) _blueprint)
      (`/Game/Characters/Gruttin/BP_Gruttin.GetRessource` (`self.As BP Gruttin`) _price)
      (break)))
  (`Actor.K2_DestroyActor` _hitactor))

(event `Key|MouseScrollUp`
  (params (Key :type "Key Structure"))
  (bind _build_index (`self.Build_Index`))
  (bind _returnvalue (- (`KismetArrayLibrary.Array_Length` (`self.DT_BuildParts`)) 1))
  ; Sélection trap par le scroll
  (:`Pressed`
    (if (`self.InBuildMode?`)
      (if (!= _build_index _returnvalue)
        (set `self.Build_Index` (`KismetMathLibrary.Clamp` (+ _build_index 1) 0 _returnvalue))
        (else
          (set `self.Build_Index` 0)))
      (`self.ResetBuildMode` :!label _label_9)
      (bind _preview_mesh (`self.Preview_Mesh`)
        (:`then`
          (`StaticMeshComponent.SetStaticMesh` _preview_mesh null)
          (set `self.Preview_Mesh` null)
          (`self.ResetBuildMode`))
        (:`else`)))))

(event `Key|MouseScrollDown`
  (params (Key :type "Key Structure"))
  (bind _returnvalue (- (`KismetArrayLibrary.Array_Length` (`self.DT_BuildParts`)) 1))
  ; Sélection trap par le scroll
  (:`Pressed`
    (if (`self.InBuildMode?`)
      (if (!= (`self.Build_Index`) 0)
        (set `self.Build_Index` (`KismetMathLibrary.Clamp` (- (`self.Build_Index`) 1) 0 _returnvalue))
        (goto _label_9)
        (else
          (set `self.Build_Index` _returnvalue)
          (goto _label_9))))))

(fn `BuildCycle`)

(fn `GiveBuildColor`)

(fn `SpawnBuildGhost`)