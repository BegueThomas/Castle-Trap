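; Base actor for player-built traps, which charges resources on placement and self-destructs with a refund when overlapping another build or resource pile.
; Contact traps damage enemies instantly or on a timer and can slow them; ranged traps use looping timers to aim and fire projectiles when a line trace confirms the target.
; Attacking wears down health, shown on a player-facing widget when targeted and repaired with resources through a timeline progress bar.
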(event `Spawn`
  (params (Price :type "Float (double-precision)"))
  (bind _overlappingactors (`self.GetOverlappingActors` "BP_BuildMaster_C"))
  (bind _overlappingactors_2 (`self.GetOverlappingActors` "/Game/Enviro/Ressource/BP_RessourcePile.BP_RessourcePile_C"))
  (`self.Spawn_function` _overlappingactors _overlappingactors Price)
  (`self.Spawn_function` _overlappingactors_2 _overlappingactors_2 Price)
  ; dépense
  (`/Game/Characters/Gruttin/BP_Gruttin.SpendRessource` (`self.As BP Gruttin`) Price))

(event `self.ReceiveTick`
  (params (DeltaSeconds :type "Float (single-precision)"))
  (bind _health_text (`self.Health_text`))
  (bind _shoot_direction (`self.Shoot_Direction`))
  (bind (_returnvalue_location _returnvalue_rotation) (`KismetMathLibrary.BreakTransform` (`SceneComponent.K2_GetComponentToWorld` _shoot_direction)))
  ; Rotation feedback vie
  (`SceneComponent.K2_SetWorldRotation` _health_text (`KismetMathLibrary.FindLookAtRotation` (`SceneComponent.K2_GetComponentLocation` _health_text) (`SceneComponent.K2_GetComponentLocation` (`Character.CapsuleComponent` (stale `self.ReceiveBeginPlay` _output_get)))) false false)
  ; Line trace prévue pour les piéges qui tire à distance
  (if (not (`self.AttackMethod`))
    (bind (_outhit _returnvalue) (`KismetSystemLibrary.LineTraceSingle` (`SceneComponent.K2_GetComponentLocation` _shoot_direction) (+ _returnvalue_location (* (`KismetMathLibrary.GetForwardVector` _returnvalue_rotation) 1000.0)) "TraceTypeQuery2"))
    (set `self.Out Hit` _outhit)
    (set `self.Trap_Trace` _returnvalue)))

(event `self.ReceiveBeginPlay`
  (set `self.Health` (`self.MaxHealth`))
  (bind _asbp_gruttin (cast `/Game/Characters/Gruttin/BP_Gruttin` (`GameplayStatics.GetPlayerPawn` 0)))
  (bind _output_get (set `self.As BP Gruttin` _asbp_gruttin)))

(event `self.Hitbox.OnComponentBeginOverlap`
  (params (OverlappedComponent :type "PrimitiveComponent Object Reference") (OtherActor :type "Actor Object Reference") (OtherComp :type "PrimitiveComponent Object Reference") (OtherBodyIndex :type Integer) (bFromSweep :type Boolean) (SweepResult :type "HitResult Structure (by ref)"))
  (if (`self.Damages?`)
    (bind _asbp_ennemy_master (cast `/Game/Characters/Ennemy/Bp_EnnemyMaster` OtherActor))
    (if (`self.AttackMethod`)
      (if (`self.DmgInstant?`)
        (`self.Effect_Target`)
        (if (`/Game/Characters/Ennemy/Bp_EnnemyMaster.Death?` _asbp_ennemy_master) :!label _label
          (`self.Remove_dead_ennemy` _asbp_ennemy_master)
          (else
            (`/Game/Characters/Ennemy/Bp_EnnemyMaster.Damage` _asbp_ennemy_master null (`self.BaseDamage`))
            (`self.Damage` null (`self.Received_Gmg`))))
        (else
          (bind _returnvalue (`KismetSystemLibrary.K2_SetTimerDelegate` (delegate `Damage_Target`) (/ (`self.Cadence_Tire`) 10.0) true))
          (set `self.Overtime_timer` _returnvalue)
          (`self.Effect_Target`))))))

(event `/Game/Characters/IBP_Damage.Damage`
  (params (Target :type "Object Object Reference") (Damage :type "Float (double-precision)"))
  (bind _output_get (set `self.Health` (- (`self.Health`) Damage)))
  (if (<= _output_get 0.0)
    (`self.K2_DestroyActor`)))

(event `Damage_Target`
  (goto _label))

(event `Effect_Target`
  (switch `/Game/Enviro/Trap/E_Effects` (`self.Effect`)
    (:`NewEnumerator1`
      (`/Game/Characters/Ennemy/Bp_EnnemyMaster.Ralenti` (stale `self.Hitbox.OnComponentBeginOverlap` _asbp_ennemy_master) 2.0 3.0))))

(event `self.Hitbox.OnComponentEndOverlap`
  (params (OverlappedComponent :type "PrimitiveComponent Object Reference") (OtherActor :type "Actor Object Reference") (OtherComp :type "PrimitiveComponent Object Reference") (OtherBodyIndex :type Integer))
  (`KismetSystemLibrary.K2_ClearAndInvalidateTimerHandle` (`self.Overtime_timer`)))

(event `/Game/Enviro/Trap/Blueprints/IBP_SeeStat.OnObjectTargeted`
  (bind _health_text (`self.Health_text`))
  ; Feedback Vie
  (`SceneComponent.SetVisibility` _health_text true false)
  (bind _asui_health_trap (cast `/Game/UI/UI_HealthTrap` (`WidgetComponent.GetWidget` _health_text)))
  (`/Game/UI/UI_HealthTrap.Stats` _asui_health_trap (`self.Health`) (`self.MaxHealth`)))

(event `/Game/Enviro/Trap/Blueprints/IBP_SeeStat.OnObjectUntargeted`
  ; Feedback Vie
  (`SceneComponent.SetVisibility` (`self.Health_text`) false false))

(event `self.Range.OnComponentBeginOverlap`
  (params (OverlappedComponent :type "PrimitiveComponent Object Reference") (OtherActor :type "Actor Object Reference") (OtherComp :type "PrimitiveComponent Object Reference") (OtherBodyIndex :type Integer) (bFromSweep :type Boolean) (SweepResult :type "HitResult Structure (by ref)"))
  (if (`self.AttackMethod`)
    _
    (elif (`|EnumEquality` (`PrimitiveComponent.GetCollisionObjectType` OtherComp) "ECC_GameTraceChannel2")
      (`KismetArrayLibrary.Array_Add` (`self.List_Target_Range`) OtherActor)
      (`KismetSystemLibrary.PrintString` "i seeeee youuuuu" true true (struct :`R` 1.0 :`B` 0.05554 :`A` 1.0))
      (bind _returnvalue (`KismetSystemLibrary.K2_SetTimerDelegate` (delegate `LookAtTarget`) 0.1 true))
      (set `self.Look_At_Handler` _returnvalue)
      (bind _returnvalue_2 (`KismetSystemLibrary.K2_SetTimerDelegate` (delegate `Attack`) (/ (`self.Cadence_Tire`) 10.0) true))
      (set `self.Shoot_Handler` _returnvalue_2))))

(event `LookAtTarget`
  (bind _shoot_direction (`self.Shoot_Direction`))
  (`SceneComponent.K2_SetWorldRotation` _shoot_direction (`KismetMathLibrary.FindLookAtRotation` (`SceneComponent.K2_GetComponentLocation` _shoot_direction) (`self.K2_GetActorLocation` (`|GetArrayItem` (`self.List_Target_Range`)))) false false))

(event `Attack`
  (if (> (`self.Health`) 0.0)
    ; Trace
    (if (`self.Trap_Trace`)
      (for _array_element (`self.List_Target_Range`)
        (bind _returnvalue (== _array_element (`.HitActor` (`GameplayStatics.BreakHitResult` (`self.Out Hit`)))))
        (if _returnvalue
          (break)))
      (if _returnvalue
        (`|SpawnActorFromClass` "/Game/Enviro/Trap/Blueprints/BP_Projectile.BP_Projectile_C" (`SceneComponent.K2_GetComponentToWorld` (`self.Shoot_Direction`)) "Undefined" "MultiplyWithRoot" null null)
        (set `self.Health` (- (`self.Health`) 1.0))))))

(event `Remove_dead_ennemy`
  (params (Item :type "Actor Object Reference (by ref)"))
  (`KismetArrayLibrary.Array_RemoveItem` (`self.List_Target_Range`) Item)
  ; Cleaar list ennemy dans la range
  (if (`KismetArrayLibrary.Array_IsEmpty` (`self.List_Target_Range`)) :!label _label_2
    (`KismetSystemLibrary.K2_ClearAndInvalidateTimerHandle` (`self.Look_At_Handler`))
    (`KismetSystemLibrary.K2_ClearAndInvalidateTimerHandle` (`self.Shoot_Handler`))))

(event `self.Range.OnComponentEndOverlap`
  (params (OverlappedComponent :type "PrimitiveComponent Object Reference") (OtherActor :type "Actor Object Reference") (OtherComp :type "PrimitiveComponent Object Reference") (OtherBodyIndex :type Integer))
  ; Cleaar list ennemy dans la range
  (`KismetArrayLibrary.Array_RemoveItem` (`self.List_Target_Range`) OtherActor)
  (goto _label_2))

(event `/Game/Characters/Gruttin/IBP_Interact.Interact`
  (bind _as_bp_gruttin (`self.As BP Gruttin`))
  (bind _returnvalue (- (`self.MaxHealth`) (`self.Health`)))
  (bind _ui_gruttin (`/Game/Characters/Gruttin/BP_Gruttin.Ui_Gruttin` (`self.As BP Gruttin`)))
  (bind _progressbar_0 (`/Game/UI/UI_Gruttin.ProgressBar_0` _ui_gruttin))
  ; Systéme de réparation
  (if (> _returnvalue 0.0)
    (set `self.Repair_Loop_Index` _returnvalue)
    (if (>= (`/Game/Characters/Gruttin/BP_Gruttin.HeldRessource` _as_bp_gruttin) 5.0)
      (`TimelineComponent.SetPlayRate` (`self.Progress_Timeline`) 1.0)
      (set `Widget.Visibility` "Visible" _progressbar_0)
      (bind (_direction _progress) (`Timeline|Progress_Timeline` :!via `PlayFromStart` :!label _label_3)
        (:`Update`
          (set `/Game/UI/UI_Gruttin.Progress` _progress _ui_gruttin))
        (:`Finished`
          (if (== _progress 1.0)
            (set `Widget.Visibility` "Hidden" _progressbar_0)
            ;; Boucle réparation
            (if (not (== (`self.Repair_Loop_Index`) 0.0)) :!label _label_4
              (`/Game/Characters/Gruttin/BP_Gruttin.SpendRessource` _as_bp_gruttin 1.0)
              (set `self.Health` (+ (`self.Health`) 1.0))
              (`KismetSystemLibrary.PrintString` "tik tik")
              (set `self.Repair_Loop_Index` (- (`self.Repair_Loop_Index`) 1.0))
              (if (>= (`/Game/Characters/Gruttin/BP_Gruttin.HeldRessource` (`self.As BP Gruttin`)) 5.0)
                (goto _label_4)))))))))

(event `/Game/Characters/Gruttin/IBP_Interact.Cancel_Intract`
  ; Systéme de réparation
  (`TimelineComponent.SetPlayRate` (`self.Progress_Timeline`) 10.0)
  (set `Widget.Visibility` "Hidden" (`/Game/UI/UI_Gruttin.ProgressBar_0` (`/Game/Characters/Gruttin/BP_Gruttin.Ui_Gruttin` (`self.As BP Gruttin`))))
  (goto _label_3 :!via `Reverse`))

(fn `Spawn_function`
  (params (Array :type "Array of Object Object Reference") (TargetArray :type "Array of Object Object Reference (by ref)") (Price :type "Float (double-precision)"))
  (for _array_element Array
    (`KismetSystemLibrary.PrintString` (`KismetSystemLibrary.GetDisplayName` _array_element)))
  (if (> (`KismetArrayLibrary.Array_Length` TargetArray) 0)
    (`KismetSystemLibrary.PrintString` "dieeeeeeee")
    (`self.K2_DestroyActor`)
    ; Remboursement
    (`/Game/Characters/Gruttin/BP_Gruttin.GetRessource` (`self.As BP Gruttin`) Price)))

(fn `UserConstructionScript`)