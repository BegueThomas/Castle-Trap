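; Resource pile that the player's BP_Gruttin draws from through a hold-to-collect interaction.
; Box overlap shows or hides the pile UI on the Gruttin's widget and sets Near, which exit never clears.
; Interact plays a progress timeline, then subtracts the player's missing capacity from the pile, unclamped, and passes it to GetRessource.
; CancelIntract rapidly reverses the timeline; Restock and BeginPlay refill to MaxPile.
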(event `/Game/Characters/Gruttin/IBP_Interact.Restock`
  (set `self.Pile_Ressource` (`self.Max_Pile`) :!label _label))

(event `self.ReceiveBeginPlay`
  (bind _asbp_gruttin (cast `/Game/Characters/Gruttin/BP_Gruttin` (`GameplayStatics.GetPlayerPawn` 0)))
  (bind _output_get (set `self.As BP Gruttin` _asbp_gruttin))
  (goto _label))

(event `self.Box.OnComponentBeginOverlap`
  (params (OverlappedComponent :type "PrimitiveComponent Object Reference") (OtherActor :type "Actor Object Reference") (OtherComp :type "PrimitiveComponent Object Reference") (OtherBodyIndex :type Integer) (bFromSweep :type Boolean) (SweepResult :type "HitResult Structure (by ref)"))
  (bind _as_bp_gruttin (`self.As BP Gruttin`))
  (bind _ui_gruttin (`/Game/Characters/Gruttin/BP_Gruttin.Ui_Gruttin` _as_bp_gruttin))
  (if (== OtherActor _as_bp_gruttin)
    (set `self.Near?` true)
    (set `Widget.Visibility` "Visible" (`/Game/UI/UI_Gruttin.ProgressBar_0` _ui_gruttin))
    (set `Widget.Visibility` "Visible" (`/Game/UI/UI_Gruttin.Ressource_amount` _ui_gruttin))
    (set `Widget.Visibility` "Visible" (`/Game/UI/UI_Gruttin.hold_text` _ui_gruttin))
    (set `/Game/UI/UI_Gruttin.Pile_R` (`self.Pile_Ressource`) _ui_gruttin)))

(event `self.Box.OnComponentEndOverlap`
  (params (OverlappedComponent :type "PrimitiveComponent Object Reference") (OtherActor :type "Actor Object Reference") (OtherComp :type "PrimitiveComponent Object Reference") (OtherBodyIndex :type Integer))
  (bind _ui_gruttin (`/Game/Characters/Gruttin/BP_Gruttin.Ui_Gruttin` (`self.As BP Gruttin`)))
  (if (== OtherActor (`self.As BP Gruttin`))
    (set `self.Near?` true)
    (set `Widget.Visibility` "Hidden" (`/Game/UI/UI_Gruttin.ProgressBar_0` _ui_gruttin))
    (set `Widget.Visibility` "Hidden" (`/Game/UI/UI_Gruttin.Ressource_amount` _ui_gruttin))
    (set `Widget.Visibility` "Hidden" (`/Game/UI/UI_Gruttin.hold_text` _ui_gruttin))))

(event `/Game/Characters/Gruttin/IBP_Interact.Interact`
  (bind _as_bp_gruttin (`self.As BP Gruttin`))
  (bind _ui_gruttin (`/Game/Characters/Gruttin/BP_Gruttin.Ui_Gruttin` (`self.As BP Gruttin`)))
  (bind _returnvalue (- (`/Game/Characters/Gruttin/BP_Gruttin.MaxRessource` _as_bp_gruttin) (`/Game/Characters/Gruttin/BP_Gruttin.HeldRessource` _as_bp_gruttin)))
  (bind _progressbar_0 (`/Game/UI/UI_Gruttin.ProgressBar_0` _ui_gruttin))
  (if (`self.Near?`)
    (if (!= (`self.Pile_Ressource`) 0.0)
      (`TimelineComponent.SetPlayRate` (`self.Progress_Timeline`) 1.0)
      (set `Widget.Visibility` "Visible" _progressbar_0)
      (bind (_direction _progress) (`Timeline|Progress_Timeline` :!via `PlayFromStart` :!label _label_2)
        (:`Update`
          (set `/Game/UI/UI_Gruttin.Progress` _progress _ui_gruttin))
        (:`Finished`
          (if (== _progress 1.0)
            (set `Widget.Visibility` "Hidden" _progressbar_0)
            (bind _output_get (set `self.Pile_Ressource` (- (`self.Pile_Ressource`) _returnvalue)))
            (set `/Game/UI/UI_Gruttin.Pile_R` _output_get (`/Game/Characters/Gruttin/BP_Gruttin.Ui_Gruttin` _as_bp_gruttin))
            (`/Game/Characters/Gruttin/BP_Gruttin.GetRessource` _as_bp_gruttin _returnvalue)))))))

(event `/Game/Characters/Gruttin/IBP_Interact.Cancel_Intract`
  (`TimelineComponent.SetPlayRate` (`self.Progress_Timeline`) 10.0)
  (set `Widget.Visibility` "Hidden" (`/Game/UI/UI_Gruttin.ProgressBar_0` (`/Game/Characters/Gruttin/BP_Gruttin.Ui_Gruttin` (`self.As BP Gruttin`))))
  (goto _label_2 :!via `Reverse`))

(fn `UserConstructionScript`)