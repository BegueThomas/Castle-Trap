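; BP_WeaponPIle is an environment actor that builds a randomly thinned pile of a single weapon mesh.
; The Construction Script assigns Weapon to every static mesh component, then destroys those whose random roll fails against ChancePercentage.
; The roll is an unseeded integer 0 or 1, so values from 0 to below 100 act as a coin flip, and 100 removes all.
; The event graph is unused.
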(fn `UserConstructionScript`
  (bind _returnvalue (`self.K2_GetComponentsByClass` "/Script/Engine.StaticMeshComponent"))
  (for (_array_element _array_index) _returnvalue
    (`StaticMeshComponent.SetStaticMesh` (`|GetArrayItem` _returnvalue _array_index) (`self.Weapon`))
    (if (not (> (`KismetMathLibrary.RandomIntegerInRange` 0 1) (/ (`self.ChancePercentage`) 100)))
      (`ActorComponent.K2_DestroyComponent` _array_element))))