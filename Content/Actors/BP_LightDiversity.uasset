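; BP_LightDiversity is an actor that varies flickering lights by randomizing their RandomIntensity values when its construction script runs.
; It gathers actors tagged with the LightTag enum's name and casts each to BP_LightFlicker.
; Each new value falls between the current one minus RandomThreshold and RandomThreshold alone, so the upper bound ignores the current value and reruns build on earlier results.
; The event graph holds only disabled placeholder events.
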(fn `UserConstructionScript`
  (bind _randomthreshold (`self.RandomThreshold`))
  (bind _outactors (`GameplayStatics.GetAllActorsWithTag` (`|GetEnumeratorName` (`self.LightTag`))))
  (for _array_element _outactors
    (bind _asbp_light_flicker (cast `/Game/Actors/BP_LightFlicker` _array_element))
    (set `/Game/Actors/BP_LightFlicker.Random_Intensity` (`KismetMathLibrary.RandomFloatInRange` (- (`/Game/Actors/BP_LightFlicker.Random_Intensity` _asbp_light_flicker) _randomthreshold) (+ 0.0 _randomthreshold)) _asbp_light_flicker)))