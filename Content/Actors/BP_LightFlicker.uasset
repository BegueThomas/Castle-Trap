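; BP_LightFlicker is a configurable point light actor that can either shine steadily or flicker.
; The construction script applies exposed color, radius, source shape and shadow settings, and sets intensity only when flickering is off.
; When flickering is on, BeginPlay creates a dynamic instance of the light function material and passes it speed, intensity and minimum, leaving the animation to the material instead of Tick.
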(event `self.ReceiveBeginPlay`
  (if (`self.IsFlickering?`)
    (bind _returnvalue (`KismetMaterialLibrary.CreateDynamicMaterialInstance` (`LightComponent.LightFunctionMaterial` (`self.PointLight`))))
    (bind _output_get (set `self.LightFunction` _returnvalue))
    (`LightComponent.SetLightFunctionMaterial` (`self.PointLight`) _output_get)
    (`MaterialInstanceDynamic.SetScalarParameterValue` (`self.LightFunction`) "FlickerSpeed" (`self.FlickerSpeed`))
    (`MaterialInstanceDynamic.SetScalarParameterValue` (`self.LightFunction`) "LightIntensity" (`self.LightIntensity`))
    (`MaterialInstanceDynamic.SetScalarParameterValue` (`self.LightFunction`) "MinIntensity" (`self.Flicker_Intensity_Min`))))

(fn `UserConstructionScript`
  ; Intensity
  (if (not (`self.IsFlickering?`))
    (`LightComponent.SetIntensity` (`self.PointLight`) (`self.LightIntensity`)))
  ; Color
  (`LightComponent.SetLightColor` (`self.PointLight`) (`KismetMathLibrary.Conv_ColorToLinearColor` (`self.LightColor`)) true)
  ; Boundaries
  (`LocalLightComponent.SetAttenuationRadius` (`self.PointLight`) (`self.AttenuationRadius`))
  (`PointLightComponent.SetSourceRadius` (`self.PointLight`) (`self.SourceRadius`))
  (`PointLightComponent.SetSoftSourceRadius` (`self.PointLight`) (`self.SoftSourceRadius`))
  (`PointLightComponent.SetSourceLength` (`self.PointLight`) (`self.SourceLenght`))
  (`LightComponentBase.SetCastShadows` (`self.PointLight`) (`self.CastShadows`)))